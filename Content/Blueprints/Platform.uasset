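; Platform actor that reacts when the player character touches its Box trigger.
; On BeginPlay it moves the Box to the relative position held in NewLocation.
; Each player overlap snaps the static mesh to zero world rotation, while a DoOnce that is never reset plays the Checked 2D sound only on the first touch.
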(event OnComponentBeginOverlap(Box)
  (params (OverlappedComponent :type Primitive%20Component%20Object%20Reference) (OtherActor :type Actor%20Object%20Reference) (OtherComp :type Primitive%20Component%20Object%20Reference) (OtherBodyIndex :type Integer) (bFromSweep :type Boolean) (SweepResult :type Hit%20Result%20Structure%20%28by%20ref%29))
  (if (== OtherActor (Game|GetPlayerCharacter 0))
    (Transformation|SetWorldRotation (Variables|Default|GetStaticMesh) "0, 0, 0" false false)
    (Utilities|FlowControl|DoOnce false
      (:Completed
        (Audio|PlaySound2D "/Engine/VREditor/Sounds/UI/Checked.Checked" 1.0 1.0 0.0 0 0)))))

(event EventBeginPlay
  (Transformation|SetRelativeLocation (Variables|Default|GetBox) (Variables|Default|GetNew%20Location) false false))

(fn ConstructionScript)