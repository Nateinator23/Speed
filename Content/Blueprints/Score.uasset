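; Score is a Blueprint that measures and displays the first-person player's speed on entering its trigger box.
; BeginPlay caches the player as BP_FirstPersonCharacter.
; The first Box overlap by that player passes a DoOnce with no reset, prints the velocity's magnitude and writes it to a TextRender, so only one reading registers.
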(event OnComponentBeginOverlap(Box)
  (params (OverlappedComponent :type Primitive%20Component%20Object%20Reference) (OtherActor :type Actor%20Object%20Reference) (OtherComp :type Primitive%20Component%20Object%20Reference) (OtherBodyIndex :type Integer) (bFromSweep :type Boolean) (SweepResult :type Hit%20Result%20Structure%20%28by%20ref%29))
  (bind _as_bp_first_person_character (Variables|Default|GetAs%20BP%20First%20Person%20Character))
  (bind _returnvalue (Transformation|GetVelocity _as_bp_first_person_character))
  (bind _returnvalue_2 (Math|Vector|VectorLength _returnvalue))
  (if (== OtherActor (Game|GetPlayerCharacter 0))
    (Utilities|FlowControl|DoOnce false
      (:Completed
        (Development|PrintString (Utilities|String|ToString(Float) _returnvalue_2))
        (Rendering|Components|TextRender|SetText (Variables|Default|GetTextRender) (Utilities|Text|ToText(Float) _returnvalue_2 "HalfToEven"))))))

(event EventBeginPlay
  (bind _asbp_first_person_character (Utilities|Casting|CastToBP_FirstPersonCharacter (Game|GetPlayerCharacter 0)))
  (Variables|Default|SetAs%20BP%20First%20Person%20Character _asbp_first_person_character))

(fn ConstructionScript)