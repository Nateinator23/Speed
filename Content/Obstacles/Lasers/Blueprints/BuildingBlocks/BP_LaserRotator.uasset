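; BP_LaserRotator is an obstacle building block that spawns a set of laser actors and can spin itself.
; BeginPlay destroys any referenced lasers, then spawns NumLasers A_Laser actors, all at the root location with zero rotation, and stores them.
; Tick adds local roll at SpinSpeed while IsSpinning, but the graph never attaches the lasers to the rotator.
; Radius-based circular placement math exists but is unconnected.
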(event EventBeginPlay
  (bind _laserreferences (Variables|Default|GetLaserReferences))
  ;[0.6159 0.6837 1] Handles Spawn Location and Angles
  (for _array_element _laserreferences
    (Actor|DestroyActor _array_element))
  (Utilities|Array|Clear _laserreferences)
  (for _index (range 0 (- (Variables|Default|GetNumLasers) 1))
    (bind _returnvalue (Game|SpawnActorfromClass "/Game/Obstacles/Lasers/Blueprints/BuildingBlocks/A_Laser.A_Laser_C" (Math|Transform|MakeTransform (+ (Transformation|GetWorldLocation (Variables|Default|GetRoot)) "0.000000,0.000000,0.000000") (Math|Rotator|MakeRotator 0.0 0.0 0.0) "1.000000,1.000000,1.000000") "AlwaysSpawn" "MultiplyWithRoot" 0 "(R=0.000000,G=0.000000,B=0.000000,A=0.000000)" 3e+03 0 0 0))
    (Utilities|Array|Add (Variables|Default|GetLaserReferences) _returnvalue)))

(event EventTick
  (params (DeltaSeconds :type Float%20%28single-precision%29))
  (if (Variables|Default|GetIsSpinning)
    (Transformation|AddActorLocalRotation (Math|Rotator|MakeRotator (* DeltaSeconds (Variables|Default|GetSpinSpeed)) 0.0 0.0) false false)))

(fn ConstructionScript)